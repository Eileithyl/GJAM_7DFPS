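; Placeable copper cable actor that the player places with the Inspect input action.
; Tick enables or disables this actor's input from player controller 0 every frame, based on PlayerCanInput.
; Pressing Inspect swaps the highlight mesh for the default mesh and prints a placed message, though it sets CopperCablePlaced to false.
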(event `self.ReceiveTick`
  (params (DeltaSeconds :type "Float (single-precision)"))
  (bind _returnvalue (`GameplayStatics.GetPlayerController` 0))
  (if (`self.PlayerCanInput?`)
    (`self.EnableInput` _returnvalue)
    (`KismetSystemLibrary.PrintString` "EnableINput")
    (else
      (`self.DisableInput` _returnvalue))))

(event `InputAction|Inspect` :consume false :overrideparent false
  (params (Key :type "Key Structure"))
  (:`Pressed`
    (`SceneComponent.SetHiddenInGame` (`self.DefaultMesh`) false false)
    (`SceneComponent.SetHiddenInGame` (`self.HighlightMesh`) true false)
    (set `self.CopperCablePlaced` false)
    (`KismetSystemLibrary.PrintString` "Copper Cable Placed")))

(fn `UserConstructionScript`
  (`parent.UserConstructionScript`))