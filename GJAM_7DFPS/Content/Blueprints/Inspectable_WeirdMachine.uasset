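; Inspectable weird machine actor that highlights and accepts the Inspect input when the player looks at it from close range.
; Tick uses a camera dot product and distance check to toggle custom depth, the highlight mesh and input.
; Inspect flip-flops between a blended close-up camera with title and description HUD, and the player view.
; If IsSpecial, exiting instead sets PullSwitch, removes the HUD and locks further inspection, leaving camera and player input unrestored.
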(event `self.ReceiveBeginPlay`
  (bind _asfirst_person_character (cast `/Game/FirstPersonBP/Blueprints/FirstPersonCharacter` (`GameplayStatics.GetPlayerCharacter` 0)))
  (set `self.FirstPersonCharacter` _asfirst_person_character))

(event `InputAction|Inspect`
  (params (Key :type "Key Structure"))
  (bind _returnvalue (`GameplayStatics.GetPlayerController` 0))
  (bind _returnvalue_2 (`GameplayStatics.GetPlayerController` 0))
  (bind _firstpersoncharacter (`self.FirstPersonCharacter`))
  (bind _posterhud (`/Game/FirstPersonBP/Blueprints/FirstPersonCharacter.PosterHUD` (`self.FirstPersonCharacter`)))
  (:`Pressed`
    (if (not (`self.PullSwitch`))
      (`/Engine/EditorBlueprintResources/StandardMacros.FlipFlop`
        (:`A`
          (`PlayerController.SetViewTargetWithBlend` _returnvalue_2 (`ActorComponent.GetOwner` (`self.Camera`)) 0.5 "VTBlend_Cubic" 0.0 false)
          (`self.DisableInput` _firstpersoncharacter _returnvalue_2)
          (`TextBlock.SetText` (`/Game/Widgets/PosterHUD.TitleText` (`/Game/FirstPersonBP/Blueprints/FirstPersonCharacter.PosterHUD` (`self.FirstPersonCharacter`))) (`KismetTextLibrary.Conv_StringToText` (`self.Object_Title`)))
          (`TextBlock.SetText` (`/Game/Widgets/PosterHUD.DescriptionText` _posterhud) (`KismetTextLibrary.Conv_StringToText` (`self.Object_Description`)))
          (`UserWidget.AddToViewport` _posterhud 0))
        (:`B`
          (if (`self.IsSpecial`)
            (if true
              (set `self.PullSwitch` true)
              (`Widget.RemoveFromParent` _posterhud :!label _label))
            (else
              (`PlayerController.SetViewTargetWithBlend` _returnvalue (`self.FirstPersonCharacter`) 0.5 "VTBlend_Cubic" 0.0 false)
              (`self.EnableInput` _firstpersoncharacter _returnvalue)
              (goto _label))))))))

(event `self.ReceiveTick`
  (params (DeltaSeconds :type "Float (single-precision)"))
  (bind _returnvalue (`GameplayStatics.GetPlayerController` 0))
  (bind _returnvalue_2 (`GameplayStatics.GetPlayerCameraManager` 0))
  (bind _highlightmesh (`self.HighlightMesh`))
  (bind _returnvalue_3 (- (`self.K2_GetActorLocation` self) (`PlayerCameraManager.GetCameraLocation` _returnvalue_2)))
  (if (>= (`KismetMathLibrary.Dot_VectorVector` (`KismetMathLibrary.Normal` _returnvalue_3) (`KismetMathLibrary.Normal` (`self.GetActorForwardVector` _returnvalue_2))) 0.96)
    (if (<= (`KismetMathLibrary.VSize` _returnvalue_3) 250.0)
      (`PrimitiveComponent.SetRenderCustomDepth` (`self.DefaultMesh`) true)
      (`SceneComponent.SetHiddenInGame` _highlightmesh false false)
      (`PrimitiveComponent.SetRenderCustomDepth` _highlightmesh true)
      (`self.EnableInput` _returnvalue)
      (else
        (`PrimitiveComponent.SetRenderCustomDepth` (`self.DefaultMesh`) false :!label _label_2)
        (`SceneComponent.SetHiddenInGame` _highlightmesh true false)
        (`PrimitiveComponent.SetRenderCustomDepth` _highlightmesh false)
        (`self.DisableInput` _returnvalue)))
    (else
      (goto _label_2))))

(fn `UserConstructionScript`)