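; Inspectable object actor that highlights itself when the player camera looks almost directly at it from close range.
; Every Tick it compares the camera manager's forward vector with the direction to the actor by dot product, then checks the distance.
; When both tests pass it enables custom depth on the default and highlight meshes and shows the highlight mesh, otherwise it reverses this.
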(event `self.ReceiveTick`
  (params (DeltaSeconds :type "Float (single-precision)"))
  (bind _returnvalue (`GameplayStatics.GetPlayerCameraManager` 0))
  (bind _highlightmesh (`self.HighlightMesh`))
  (bind _returnvalue_2 (- (`self.K2_GetActorLocation` self) (`PlayerCameraManager.GetCameraLocation` _returnvalue)))
  (if (>= (`KismetMathLibrary.Dot_VectorVector` (`KismetMathLibrary.Normal` _returnvalue_2) (`KismetMathLibrary.Normal` (`self.GetActorForwardVector` _returnvalue))) 0.99)
    (if (<= (`KismetMathLibrary.VSize` _returnvalue_2) 250.0)
      (`PrimitiveComponent.SetRenderCustomDepth` (`self.DefaultMesh`) true)
      (`SceneComponent.SetHiddenInGame` _highlightmesh false false)
      (`PrimitiveComponent.SetRenderCustomDepth` _highlightmesh true)
      (else
        (`PrimitiveComponent.SetRenderCustomDepth` (`self.DefaultMesh`) false :!label _label)
        (`SceneComponent.SetHiddenInGame` _highlightmesh true false)
        (`PrimitiveComponent.SetRenderCustomDepth` _highlightmesh false)))
    (else
      (goto _label))))

(fn `UserConstructionScript`)