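; Placeable copper cable spot that the player fills by pressing Inspect, provided the character has moved the poster and owns the copper wire.
; Tick calls the parent, then enables or disables the actor's input each frame based on PlayerCanInput.
; A successful placement unhides the default mesh, hides the highlight mesh, sets CopperCablePlaced and prints a confirmation.
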(event `self.ReceiveTick`
  (params (DeltaSeconds :type "Float (single-precision)"))
  (bind _returnvalue (`GameplayStatics.GetPlayerController` 0))
  (`parent.ReceiveTick` 0.0)
  (if (`self.PlayerCanInput?`)
    (`self.EnableInput` _returnvalue)
    (else
      (`self.DisableInput` _returnvalue))))

(event `InputAction|Inspect` :consume false :overrideparent false
  (params (Key :type "Key Structure"))
  (:`Pressed`
    (bind _asfirst_person_character (cast `/Game/FirstPersonBP/Blueprints/FirstPersonCharacter` (`GameplayStatics.GetPlayerCharacter` 0)))
    (if (`/Game/FirstPersonBP/Blueprints/FirstPersonCharacter.PosterMoved?` _asfirst_person_character)
      (if (`/Game/FirstPersonBP/Blueprints/FirstPersonCharacter.CopperWireOwned` _asfirst_person_character)
        (`SceneComponent.SetHiddenInGame` (`self.DefaultMesh`) false false)
        (`SceneComponent.SetVisibility` (`self.HighlightMesh`) false false)
        (set `self.CopperCablePlaced` true)
        (`KismetSystemLibrary.PrintString` "Copper Cable Placed")))))

(fn `UserConstructionScript`
  (`parent.UserConstructionScript`))