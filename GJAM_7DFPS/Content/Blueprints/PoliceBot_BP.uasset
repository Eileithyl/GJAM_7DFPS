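; Police robot NPC that greets the player and delivers a scripted briefing on a missing carriage passenger.
; A box overlap triggers the greeting, resetting on exit, while a nested DoOnce limits the briefing to one run.
; The briefing chains Delays to sequence RobotDialogue widget subtitles with robot voice sounds, toggling IsTalking on the AnimBP.
; When it finishes, it unblocks the player's inspection and sets movement to Walking.
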(event `self.ReceiveBeginPlay`
  (bind _asfirst_person_character (cast `/Game/FirstPersonBP/Blueprints/FirstPersonCharacter` (`GameplayStatics.GetPlayerCharacter` 0)))
  (set `self.FirstPersonCharacter` _asfirst_person_character)
  (bind _returnvalue (`|CreateWidget` "/Game/Widgets/RobotDialogue.RobotDialogue_C"))
  (set `self.RobotDialogue` _returnvalue)
  (`self.EnableInput` (`GameplayStatics.GetPlayerController` 0)))

(event `self.Box.OnComponentBeginOverlap`
  (params (OverlappedComponent :type "PrimitiveComponent Object Reference") (OtherActor :type "Actor Object Reference") (OtherComp :type "PrimitiveComponent Object Reference") (OtherBodyIndex :type Integer) (bFromSweep :type Boolean) (SweepResult :type "HitResult Structure (by ref)"))
  (bind _robotdialogue (`self.RobotDialogue`))
  (set `self.PlayerIsNearby` true)
  (`/Engine/EditorBlueprintResources/StandardMacros.DoOnce` false :!label _label
    (:`Completed`
      (if (`self.PlayIntro?`)
        (`KismetSystemLibrary.Delay` 2.0))
      (`UserWidget.AddToViewport` _robotdialogue 0)
      (`GameplayStatics.PlaySound2D` "/Game/Audio/robovoice_detective.robovoice_detective" 0.1 1.0 0.0 null null)
      (set `/Game/Widgets/RobotDialogue.RobotDialogueText` " \"Detective?\"" _robotdialogue)
      (`/Engine/EditorBlueprintResources/StandardMacros.DoOnce` false
        (:`Completed`
          (`self.IntroDIalogue`))))))

(event `self.Box.OnComponentEndOverlap`
  (params (OverlappedComponent :type "PrimitiveComponent Object Reference") (OtherActor :type "Actor Object Reference") (OtherComp :type "PrimitiveComponent Object Reference") (OtherBodyIndex :type Integer))
  (set `self.PlayerIsNearby` false)
  (`Widget.RemoveFromParent` (`self.RobotDialogue`))
  (set `self.PlayIntro?` false)
  (goto _label :!via `Reset`))

(event `IntroDIalogue`
  (bind _robotdialogue (`self.RobotDialogue`))
  (bind _robotdialogue_2 (`self.RobotDialogue`))
  (bind _robotdialogue_3 (`self.RobotDialogue`))
  (bind _robotdialogue_4 (`self.RobotDialogue`))
  (bind _robotdialogue_5 (`self.RobotDialogue`))
  (bind _robotdialogue_6 (`self.RobotDialogue`))
  (bind _robotdialogue_7 (`self.RobotDialogue`))
  (bind _robotdialogue_8 (`self.RobotDialogue`))
  (`KismetSystemLibrary.Delay` 2.0)
  (bind _aspolice_bot_anim_bp (cast `/Game/Blueprints/PoliceBot_AnimBP` (`SkeletalMeshComponent.GetAnimInstance` (`self.Mesh`))))
  (set `/Game/Blueprints/PoliceBot_AnimBP.IsTalking?` true _aspolice_bot_anim_bp)
  (`Widget.RemoveFromParent` (`self.RobotDialogue`))
  (`GameplayStatics.PlaySound2D` "/Game/Audio/robovoice_mid.robovoice_mid" 0.1 1.0 0.0 null null)
  (set `/Game/Widgets/RobotDialogue.RobotDialogueText` " \"Hmm. \nI didn't think there were any more \nhuman detectives around…\"" _robotdialogue_7)
  (`UserWidget.AddToViewport` _robotdialogue_7 0)
  (`KismetSystemLibrary.Delay` 5.0)
  (`Widget.RemoveFromParent` _robotdialogue_7)
  (`GameplayStatics.PlaySound2D` "/Game/Audio/robovoice_long.robovoice_long" 0.1 1.0 0.0 null null)
  (set `/Game/Widgets/RobotDialogue.RobotDialogueText` " “I’m to fill you in... \nThere were five passengers riding the carriage”" _robotdialogue_3)
  (`UserWidget.AddToViewport` _robotdialogue_3 0)
  (`KismetSystemLibrary.Delay` 7.0)
  (`Widget.RemoveFromParent` _robotdialogue_3)
  (`GameplayStatics.PlaySound2D` "/Game/Audio/robovoice_afterthought.robovoice_afterthought" 0.1 1.0 0.0 null null)
  (set `/Game/Widgets/RobotDialogue.RobotDialogueText` " “Only four injured were removed”" _robotdialogue_8)
  (`UserWidget.AddToViewport` _robotdialogue_8 0)
  (`KismetSystemLibrary.Delay` 4.0)
  (`Widget.RemoveFromParent` _robotdialogue_8)
  (`GameplayStatics.PlaySound2D` "/Game/Audio/robovoice_mid.robovoice_mid" 0.1 1.0 0.0 null null)
  (set `/Game/Widgets/RobotDialogue.RobotDialogueText` " “One is missing. \nPolice scans indicate an accident of sorts”" _robotdialogue_2)
  (`UserWidget.AddToViewport` _robotdialogue_2 0)
  (`KismetSystemLibrary.Delay` 6.0)
  (`Widget.RemoveFromParent` _robotdialogue_2)
  (`GameplayStatics.PlaySound2D` "/Game/Audio/robovoice_short.robovoice_short" 0.1 1.0 0.0 null null)
  (set `/Game/Widgets/RobotDialogue.RobotDialogueText` " “Probably a malfunction somewhere”" _robotdialogue_4)
  (`UserWidget.AddToViewport` _robotdialogue_4 0)
  (`KismetSystemLibrary.Delay` 4.0)
  (`Widget.RemoveFromParent` _robotdialogue_4)
  (`KismetSystemLibrary.Delay` 1.0)
  (`GameplayStatics.PlaySound2D` "/Game/Audio/robovoice_long.robovoice_long" 0.1 1.0 0.0 null null)
  (set `/Game/Widgets/RobotDialogue.RobotDialogueText` " “You’re only here because you were traced \nto have had recent contact with the missing individual”" _robotdialogue_5)
  (`UserWidget.AddToViewport` _robotdialogue_5 0)
  (`KismetSystemLibrary.Delay` 7.0)
  (`Widget.RemoveFromParent` _robotdialogue_5)
  (`GameplayStatics.PlaySound2D` "/Game/Audio/robovoice_afterthought.robovoice_afterthought" 0.1 1.0 0.0 null null)
  (set `/Game/Widgets/RobotDialogue.RobotDialogueText` " “Which is suspicious in itself… detective”" _robotdialogue)
  (`UserWidget.AddToViewport` _robotdialogue 0)
  (`KismetSystemLibrary.Delay` 5.0)
  (`Widget.RemoveFromParent` _robotdialogue)
  (`KismetSystemLibrary.Delay` 1.0)
  (`GameplayStatics.PlaySound2D` "/Game/Audio/robovoice_long.robovoice_long" 0.1 1.0 0.0 null null)
  (set `/Game/Widgets/RobotDialogue.RobotDialogueText` " “You can add that piece of evidence to the table behind you. \nThank you very much”" _robotdialogue_6)
  (`UserWidget.AddToViewport` _robotdialogue_6 0)
  (`KismetSystemLibrary.Delay` 5.0)
  (bind _aspolice_bot_anim_bp_2 (cast `/Game/Blueprints/PoliceBot_AnimBP` (`SkeletalMeshComponent.GetAnimInstance` (`self.Mesh`))))
  (set `/Game/Blueprints/PoliceBot_AnimBP.IsTalking?` false _aspolice_bot_anim_bp_2)
  (set `/Game/FirstPersonBP/Blueprints/FirstPersonCharacter.BlockInspect` false (`self.FirstPersonCharacter`))
  (`CharacterMovementComponent.SetMovementMode` (`Character.CharacterMovement` (`self.FirstPersonCharacter`)) "MOVE_Walking" 0))

(fn `UserConstructionScript`)